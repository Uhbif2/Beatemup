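; BP_FiredComboWidget is a Blueprint that shows a fired-combo score popup through a Widget component and awards its points.
; On BeginPlay it plays the achievement sound and passes the point count, multiplier and drop timer to the WB_FiredCombo widget.
; It then adds points times multiplier to AllPoints on the player's BP_Excavator_2, so scoring depends on the widget cast succeeding.
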(event `self.ReceiveBeginPlay`
  (`GameplayStatics.PlaySound2D` "/Game/Sounds/AchievePoints.AchievePoints" 1.0 1.0 0.0 null null)
  (bind _aswb_fired_combo (cast `/Game/Oven/WB_FiredCombo` (`WidgetComponent.GetWidget` (`self.Widget`))))
  (set `/Game/Oven/WB_FiredCombo.NumPoints` (`self.Num Points`) _aswb_fired_combo)
  (set `/Game/Oven/WB_FiredCombo.PointsMultilpicator` (`self.Points Multilpicator`) _aswb_fired_combo)
  (set `/Game/Oven/WB_FiredCombo.Timer` (`self.TimeToSumm&Drop`) _aswb_fired_combo)
  (bind _asbp_excavator_2 (cast `/Game/Excavator/BP_Excavator_2` (`GameplayStatics.GetPlayerCharacter` 0)))
  (set `/Game/Excavator/BP_Excavator_2.AllPoints` (+ (* (`self.Num Points`) (`self.Points Multilpicator`)) (`/Game/Excavator/BP_Excavator_2.AllPoints` _asbp_excavator_2)) _asbp_excavator_2))

(fn `UserConstructionScript`)