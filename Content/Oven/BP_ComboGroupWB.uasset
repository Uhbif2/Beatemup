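; Actor Blueprint that displays a combo group count through a WB_GroupCombo widget hosted in its Widget component.
; On BeginPlay it copies HowMuchGroup into the widget.
; The Change_Text event calls the widget's Check with the current count when the two values differ.
; An unconnected leftover chain resets points and a timer and touches the BP_Excavator_2 player's AllPoints, but never runs.
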(event `self.ReceiveBeginPlay`
  (bind _aswb_group_combo (cast `/Game/Oven/WB_GroupCombo` (`WidgetComponent.GetWidget` (`self.Widget`))))
  (set `/Game/Oven/WB_GroupCombo.HowMuchGroup` (`self.HowMuchGroup`) _aswb_group_combo))

(event `Change_Text`
  (bind _aswb_group_combo (cast `/Game/Oven/WB_GroupCombo` (`WidgetComponent.GetWidget` (`self.Widget`))))
  (if (not (== (`self.HowMuchGroup`) (`/Game/Oven/WB_GroupCombo.HowMuchGroup` _aswb_group_combo)))
    (`/Game/Oven/WB_GroupCombo.Check` _aswb_group_combo (`self.HowMuchGroup`))))

(fn `UserConstructionScript`)