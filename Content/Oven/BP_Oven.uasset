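; BP_Oven is a furnace that destroys stunned BP_StPanel_3 enemies in its Cube volume, with fire and smoke effects.
; Each burn spawns panel parts, broadcasts points that grow with the square of the batch size, and shows floating score and group-combo actors.
; When no enemies remain, it pauses the game and opens the end-level widget.
; The combo timer's start and stop logic is disconnected.
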(event `self.ReceiveBeginPlay`
  (`|ExecutionSequence`
    (:`then_0`
      (`KismetSystemLibrary.Delay` (`KismetMathLibrary.RandomFloatInRange` 0.0 3.0))
      (`TimelineComponent.SetPlayRate` (`self.Timeline_0`) 0.7)
      (bind (_direction _newtrack_0) (`Timeline|Timeline_0` :!via `PlayFromStart`)
        (:`Update`
          (`SceneComponent.K2_SetRelativeRotation` (`self.Door`) (`KismetMathLibrary.RLerp` (struct :`Pitch` 20.0) (struct :`Pitch` 45.0) _newtrack_0) false false))))
    (:`then_1`
      (bind _asbp_excavator_2 (cast `/Game/Excavator/BP_Excavator_2` (`GameplayStatics.GetPlayerCharacter` 0)))
      (set `self.BP Excavator 2` _asbp_excavator_2))))

(event `self.ReceiveTick`
  (params (DeltaSeconds :type "Float (single-precision)"))
  (bind _returnvalue (`GameplayStatics.GetPlayerController` 0))
  (bind _howmuchgroups (`self.HowMuchGroups`))
  (bind _overlappingactors (`PrimitiveComponent.GetOverlappingActors` (`self.Cube`) "/Game/Vampire-Panels/BP_StPanel_3.BP_StPanel_3_C"))
  (bind _overlappingactors_2 (`PrimitiveComponent.GetOverlappingActors` (`self.Cube`) "/Game/Vampire-Panels/BP_StPanel_3.BP_StPanel_3_C"))
  (`|ExecutionSequence`
    (:`then_0`
      (if (`KismetArrayLibrary.Array_IsNotEmpty` _overlappingactors)
        (bind _asbp_st_panel_3 (cast `/Game/Vampire-Panels/BP_StPanel_3` (`|GetArrayItem` _overlappingactors)))
        (if (`/Game/Vampire-Panels/BP_StPanel_3.IsInStan` _asbp_st_panel_3)
          ;[1 1 1] Подсчёт врагов в группе и их уничножение.
          (set `self.HowMuchEnemy` (+ (`self.HowMuchEnemy`) (`KismetArrayLibrary.Array_Length` _overlappingactors_2)) :!label _label)
          (`self.K2_DestroyActor` _overlappingactors_2)
          (`ActorComponent.Activate` (`self.DeadlyFire`) false)
          ; Спавн куска панельки
          (bind _object_transform (`self.Spawn Some object`))
          (`|ExecutionSequence`
            (:`then_1`
              (`|SpawnActorFromClass` "/Game/VFX/BP_PanelPart.BP_PanelPart_C" _object_transform "Undefined" "MultiplyWithRoot" null null :!label _label_2)
              (`|ExecutionSequence`
                (:`then_0`
                  (`AudioComponent.Play` (`self.PanelsInFire`) 0.0)
                  ;[1 1 1] Периуд подсчёта группы. Объеденение Execution пути.
                  (`KismetSystemLibrary.Delay` 1.3)
                  (`ActorComponent.Deactivate` (`self.DeadlyFire`))
                  (`|ExecutionSequence`
                    (:`then_0`
                      ;[1 1 1] Подсчёт очков одного врага.
                      (set `self.PointsOfOneEnemy` (* (`self.HowMuchEnemy`) 100))
                      ;[1 1 1] Перевод счётчика врагов их абсолютный подсчёт для этой печи.
                      (set `self.AbsoluteEnemyCounter` (+ (`self.HowMuchEnemy`) (`self.AbsoluteEnemyCounter`)))
                      (`self.FiredEnemies` (* (`self.PointsOfOneEnemy`) (`self.HowMuchEnemy`)))
                      (`|ExecutionSequence`
                        (:`then_0`
                          (`KismetSystemLibrary.RetriggerableDelay` (* 0.25 (`self.AbsoluteEnemyCounter`)))
                          (goto _label_3 :!via `Reset`))
                        (:`then_1`
                          (`/Engine/EditorBlueprintResources/StandardMacros.DoOnce` false :!label _label_3
                            (:`Completed`
                              (bind _counter (`/Engine/EditorBlueprintResources/StandardMacros.Do N` (`self.AbsoluteEnemyCounter`) :!label _label_4)
                                (:`Exit`
                                  (bind _returnvalue_2 (`|SpawnActorFromClass` "/Game/Oven/BP_FiredComboWidget.BP_FiredComboWidget_C" (`KismetMathLibrary.MakeTransform` (0.0 0.0 0.0)) "Undefined" "MultiplyWithRoot" null 5.0 (`self.PointsOfOneEnemy`) (`KismetMathLibrary.SelectInt` _howmuchgroups 1 (> _howmuchgroups 1)) null))
                                  (`self.K2_AttachToComponent` _returnvalue_2 (`self.Soket`) "None" "SnapToTarget" "KeepRelative" "KeepRelative" true)
                                  (`self.K2_AddActorLocalOffset` _returnvalue_2 (`KismetMathLibrary.MakeVector` 0.0 0.0 (`KismetMathLibrary.Conv_IntToDouble` (* _counter -70000))) false true)
                                  (`Timeline|Timeline` :!via `PlayFromStart`
                                    (:`Update`
                                      (`SceneComponent.K2_AddLocalOffset` (`self.Soket`) (`KismetMathLibrary.MakeVector` 0.0 0.0 (* (`GameplayStatics.GetWorldDeltaSeconds`) 60.0 1.0)) false false))
                                    (:`Finished`
                                      (`KismetSystemLibrary.Delay` 0.2)
                                      (goto _label_4))))))))
                        (:`then_2`
                          (`KismetSystemLibrary.Delay` 0.2)
                          (set `self.HowMuchEnemy` 0))
                        (:`then_3`
                          ;[1 1 1 0.5] Конец уровня
                          (bind _outactors (`GameplayStatics.GetAllActorsOfClass` "/Game/Vampire-Panels/BP_StPanel_3.BP_StPanel_3_C"))
                          (if (`KismetArrayLibrary.Array_IsEmpty` _outactors)
                            (`KismetSystemLibrary.Delay` 3.0)
                            (`GameplayStatics.SetGamePaused` true)
                            (set `PlayerController.bShowMouseCursor` true _returnvalue)
                            (`WidgetBlueprintLibrary.SetInputMode_GameAndUIEx` _returnvalue null)
                            (bind _asbp_excavator_2 (cast `/Game/Excavator/BP_Excavator_2` (`GameplayStatics.GetPlayerCharacter` 0)))
                            (`/Game/Excavator/BP_Excavator_2.Stop Timer` _asbp_excavator_2)
                            (bind _returnvalue_3 (`|CreateWidget` "/Game/Interface/WB_EndLevel.WB_EndLevel_C"))
                            (set `/Game/Interface/WB_EndLevel.CharRef` _asbp_excavator_2 _returnvalue_3)
                            (`UserWidget.AddToViewport` _returnvalue_3 0)))))
                    (:`then_1`
                      (bind _result (`/Engine/EditorBlueprintResources/StandardMacros.IncrementInt` (`self.HowMuchGroups`))
                        (:`  `
                          (bind _output_get (set `self.HowMuchGroups` _result))
                          (if (> (`self.HowMuchGroups`) 1)
                            (bind _returnvalue_4 (`|SpawnActorFromClass` "/Game/Oven/BP_ComboGroupWB.BP_ComboGroupWB_C" (`KismetMathLibrary.MakeTransform` (0.0 0.0 0.0)) "Undefined" "MultiplyWithRoot" null (`self.HowMuchGroups`) null))
                            (`/Game/Oven/BP_ComboGroupWB.Change_Text` _returnvalue_4)
                            (set `self.BP_ComboGroup_WB` _returnvalue_4)
                            (`self.K2_AttachToComponent` _returnvalue_4 (`self.GroupSocet`) "None" "SnapToTarget" "KeepRelative" "KeepRelative" true))
                          (`self.Start Timer`))))))
                (:`then_1`
                  (bind (_direction _newtrack_0) (`Timeline|Smoke` :!label _label_5)
                    (:`Update`
                      (`NiagaraComponent.SetVariableFloat` (`self.Pipe smoke1`) "UniformCurveScale" _newtrack_0)
                      (`NiagaraComponent.SetVariableFloat` (`self.Pipe smoke`) "UniformCurveScale" _newtrack_0))
                    (:`Finished`
                      (`KismetSystemLibrary.Delay` 0.2)
                      (goto _label_5 :!via `SetNewTime`))))))
            (:`then_2`
              (goto _label_2))
            (:`then_3`
              (if (`KismetMathLibrary.RandomBool`)
                (goto _label_2)))))))
    (:`then_1`
      (`/Engine/EditorBlueprintResources/StandardMacros.Gate` true
        (:`Exit`
          (set `/Game/Excavator/BP_Excavator_2.ComboTimer` (`KismetSystemLibrary.K2_GetTimerRemainingTimeHandle` (`self.Timer Handle`)) (`self.BP Excavator 2`)))))))

(event `self.Cube.OnComponentBeginOverlap`
  (params (OverlappedComponent :type "PrimitiveComponent Object Reference") (OtherActor :type "Actor Object Reference") (OtherComp :type "PrimitiveComponent Object Reference") (OtherBodyIndex :type Integer) (bFromSweep :type Boolean) (SweepResult :type "HitResult Structure (by ref)"))
  (bind _asbp_st_panel_3 (cast `/Game/Vampire-Panels/BP_StPanel_3` OtherActor))
  (`/Engine/EditorBlueprintResources/StandardMacros.IsValid` _asbp_st_panel_3
    (:`Is Valid`
      (if (`/Game/Vampire-Panels/BP_StPanel_3.IsInStan` _asbp_st_panel_3)
        (goto _label)))))

(event `Start Timer`)

(event `Stop timer`)

(fn `Spawn Some object`
  (returns (`Object Transform` :type "Transform Structure"))
  (return (`KismetMathLibrary.MakeTransform` (+ (+ (* (`self.GetActorForwardVector`) 1000.0) (.location (`self.GetTransform`))) (0.0 0.0 500.0)) (.rotation (`self.GetTransform`)) (.scale (`self.GetTransform`)))))

(fn `UserConstructionScript`)