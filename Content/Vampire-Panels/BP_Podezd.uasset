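; BP_Podezd is a child Blueprint, apparently a panel-building section, of a parent handling group calculation, enemy pushing, punches and player hits.
; Its gameplay overrides only forward to that parent.
; Tick adds a debug-drawn visibility line trace along world +X from above the HighestFloor component.
; The branch printing whether the trace hit is disconnected, so the result is unused.
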(event `self.ReceiveTick`
  (params (DeltaSeconds :type "Float (single-precision)"))
  (bind _returnvalue (+ (`SceneComponent.K2_GetComponentLocation` (`self.Highest floor`)) (0.0 0.0 450.0)))
  (`parent.ReceiveTick` DeltaSeconds)
  (bind _outhit (`KismetSystemLibrary.LineTraceSingle` :`Start` _returnvalue :`End` (+ _returnvalue (5000.0 0.0 0.0)) :`TraceChannel` "TraceTypeQuery1" :`DrawDebugType` "ForOneFrame")))

(fn `CaltulateGroup_IsInGroup&GroupVector`
  (`parent.CaltulateGroup_IsInGroup&GroupVector`))

(fn `HitWithPlayer`
  (params (BP_Excavator2 :type "/Game/Excavator/BP_Excavator_2 Object Reference"))
  (`parent.HitWithPlayer` BP_Excavator2))

(fn `PunchFromBall`
  (params (BallSpeed :type "Float (double-precision)") (BallWorldLocation :type "Vector Structure"))
  (`parent.PunchFromBall` BallSpeed BallWorldLocation))

(fn `PunchPlayer`
  (params (Player :type "/Game/Excavator/BP_Excavator_2 Object Reference (by ref)"))
  (`parent.PunchPlayer` Player)
  (return))

(fn `PushOfTheNearEnemies`
  (`parent.PushOfTheNearEnemies`))

(fn `UserConstructionScript`)