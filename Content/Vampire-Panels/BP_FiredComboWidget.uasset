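; Fired-combo score display that awards combo points to the player when it begins play.
; On BeginPlay it passes its point count, multiplier and drop-sum time into the WB_FiredCombo hosted by its Widget component.
; It then adds points times multiplier to the Allpoints total on the player's BP_Excavator_2 character.
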(event `self.ReceiveBeginPlay`
  (bind _aswb_fired_combo (cast `/Game/Vampire-Panels/WB_FiredCombo` (`WidgetComponent.GetWidget` (`self.Widget`))))
  (bind _output_get (set `/Game/Vampire-Panels/WB_FiredCombo.NumPoints` (`self.Num Points`) _aswb_fired_combo))
  (bind _output_get_2 (set `/Game/Vampire-Panels/WB_FiredCombo.PointsMultilpicator` (`self.Points Multilpicator`) _aswb_fired_combo))
  (set `/Game/Vampire-Panels/WB_FiredCombo.Timer` (`self.TimeToSumm&Drop`) _aswb_fired_combo)
  (bind _asbp_excavator_2 (cast `/Game/Excavator/BP_Excavator_2` (`GameplayStatics.GetPlayerCharacter` 0)))
  (set `/Game/Excavator/BP_Excavator_2.Allpoints` (+ (* _output_get _output_get_2) (`/Game/Excavator/BP_Excavator_2.Allpoints` _asbp_excavator_2)) _asbp_excavator_2))

(fn `UserConstructionScript`)