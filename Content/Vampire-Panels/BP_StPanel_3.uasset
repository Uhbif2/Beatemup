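; Enemy character, a walking panel building with randomized walls, that chases the player in grid-like crowds and damages and knocks them back on contact.
; Tick drives AI movement, nudges overlapping panels into axis-aligned formation, and computes a group vector from visible neighbours to slow front-rankers.
; Player punches slow its walking; a punch outside large groups launches and stuns it, while stunned panels push apart to spread along one axis.
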(event `self.ReceiveBeginPlay`
  (`|ExecutionSequence`
    (:`then_0`
      (`AudioComponent.Play` (`self.PanelsWalking`) (`KismetMathLibrary.RandomFloatInRange` 0.0 1.0)))
    (:`then_1`
      ;[1 1 1] Уменьшение скорости передвижения во время ударов игрока
      (bind _asbp_excavator_2 (cast `/Game/Excavator/BP_Excavator_2` (`GameplayStatics.GetPlayerCharacter` 0)))
      (add `/Game/Excavator/BP_Excavator_2.StartPunch` _asbp_excavator_2 (delegate `StartSlowMoving`)))))

(event `StartSlowMoving`
  (params (TimerToMoveSlow :type "Float (double-precision)"))
  (bind _standartspeed (`self.StandartSpeed`))
  ;[1 1 1] Уменьшение скорости передвижения во время ударов игрока
  (`|ExecutionSequence`
    (:`then_0`
      (set `self.IsNowSlowed?` true)
      (bind (_direction _newtrack_0) (`Timeline|Timeline_0` :!via `PlayFromStart`)
        (:`Update`
          (set `CharacterMovementComponent.MaxWalkSpeed` (`KismetMathLibrary.Lerp` _standartspeed (- _standartspeed 400.0) _newtrack_0) (`self.CharacterMovement`)))))
    (:`then_1`
      (`KismetSystemLibrary.Delay` TimerToMoveSlow)
      (set `CharacterMovementComponent.MaxWalkSpeed` (`self.StandartSpeed`) (`self.CharacterMovement`))
      (set `self.IsNowSlowed?` false))))

(event `PunchWithDelay`
  (params (VectorPunch :type "Vector Structure") (PunchActor :type "Actor Object Reference"))
  (bind _returnvalue (`KismetMathLibrary.SelectFloat` (`KismetMathLibrary.RandomFloatInRange` -15.0 -7.0) (`KismetMathLibrary.RandomFloatInRange` 7.0 15.0) (`KismetMathLibrary.RandomBool`)))
  ;[1 1 1 1 22] Эвент, которые переводит врага в состояние стана.
  ;
  ; Верхняя часть секверенса толкает врага в сторону,
  ; которую принимает эвент, то есть направление
  ; коллизии, которую создаёт игрок при ударе.
  ;
  ; (Тут хорошо бы сделать код для широко удара,
  ; по логике похожий на стабилизацию линии в ударе длинным.
  ; — на основе GroupVector, понимать находиться ли враг в линии
  ; относительно вектора широкого удара, и если нет, то толкать его сильнее)
  (if (not (`self.IsInGroup`))
    (`|ExecutionSequence`
      (:`then_0`
        (`KismetSystemLibrary.Delay` 0.4)
        (set `self.LocalPunchAddVector` _returnvalue))
      (:`then_1`
        (set `self.LocalPunchAddVector` _returnvalue)
        (set `self.LastPunchVector` VectorPunch)
        (`Timeline|Timeline` :!via `PlayFromStart`
          (:`Update`
            (if (`PrimitiveComponent.IsOverlappingActor` (`self.CapsuleComponent`) PunchActor)
              (`self.LaunchCharacter` (`KismetMathLibrary.GreaterGreater_VectorRotator` (* (`GameplayStatics.GetWorldDeltaSeconds`) VectorPunch 6.0) (`KismetMathLibrary.MakeRotator` 0.0 0.0 (`self.LocalPunchAddVector`))))))))
      (:`then_2`
        (`self.ToStanWithTimer` 5.0))
      (:`then_3`
        (`KismetSystemLibrary.Delay` (`KismetMathLibrary.RandomFloatInRange` 0.0 0.3))
        (`GameplayStatics.PlaySound2D` "/Game/Sounds/AttackWithBreak.AttackWithBreak" 1.0 1.0 0.0 null null)))))

(event `ToStanWithTimer`
  (params (TimerToOutOfStan :type "Float (double-precision)" :default 5.0))
  (bind _box (`self.Box`))
  (bind _capsulecomponent (`self.CapsuleComponent`))
  ;[1 1 1 1 22] Эвент, которые переводит врага в состояние стана.
  ;
  ; Верхняя часть секверенса толкает врага в сторону,
  ; которую принимает эвент, то есть направление
  ; коллизии, которую создаёт игрок при ударе.
  ;
  ; (Тут хорошо бы сделать код для широко удара,
  ; по логике похожий на стабилизацию линии в ударе длинным.
  ; — на основе GroupVector, понимать находиться ли враг в линии
  ; относительно вектора широкого удара, и если нет, то толкать его сильнее)
  (`|ExecutionSequence`
    (:`then_0`
      (set `self.IsInStan` true)
      (`PrimitiveComponent.SetCollisionEnabled` _box "NoCollision")
      (`CapsuleComponent.SetCapsuleRadius` _capsulecomponent 25.0 false)
      (`KismetSystemLibrary.Delay` 0.4)
      (`|ExecutionSequence`
        (:`then_0`
          (`CapsuleComponent.SetCapsuleRadius` (`self.CapsuleComponent`) 30.0 true :!label _label)
          (`CapsuleComponent.SetCapsuleRadius` (`self.CapsuleComponent`) 40.0 true)
          (`KismetSystemLibrary.Delay` 0.1)
          (`/Engine/EditorBlueprintResources/StandardMacros.Gate` false :!label _label_2
            (:`Exit`
              (goto _label))))
        (:`then_1`
          (goto _label_2 :!via `Open`))))
    (:`then_1`
      (`KismetSystemLibrary.RetriggerableDelay` TimerToOutOfStan)
      (set `self.IsInStan` false)
      (`PrimitiveComponent.SetCollisionEnabled` _box "QueryAndPhysics")
      (`CapsuleComponent.SetCapsuleRadius` _capsulecomponent 40.0 true)
      (goto _label_2 :!via `Close`))))

(event `self.ReceiveTick`
  (params (DeltaSeconds :type "Float (single-precision)"))
  (bind _returnvalue_location (`KismetMathLibrary.BreakTransform` (`self.GetTransform`)))
  (bind _charactermovement (`self.CharacterMovement`))
  (bind _panelswalking (`self.PanelsWalking`))
  (bind (_returnvalue_x _returnvalue_y) (`KismetMathLibrary.BreakVector` (`self.K2_GetActorLocation` self)))
  (bind (_returnvalue_x_2 _returnvalue_y_2) (`KismetMathLibrary.BreakVector` (`SceneComponent.GetForwardVector` (`self.CapsuleComponent`))))
  (bind _velocity (`MovementComponent.Velocity` (`self.CharacterMovement`)))
  (`|ExecutionSequence`
    (:`then_0`
      ;[1 1 1] Код, которые задаёт искуственому интелекту врагу куда ходить.
      ;
      ; Так сложно, чтобы враги не застревали в друг-друге при передвижении в линии на игрока.
      (if (`self.IsInStan`)
        ;;[1 1 1] Код, которые останавливает AI движение врага.
        (`|AIMoveTo` self _returnvalue_location null
          (:`then`
            (`AudioComponent.SetVolumeMultiplier` _panelswalking 0.0)))
        (else
          (`KismetSystemLibrary.Delay` 0.2)
          (if (`self.IsCanMove?`)
            (`|AIMoveTo` self (`self.AI Destination Calculate`) null
              (:`then`
                (`AudioComponent.SetVolumeMultiplier` _panelswalking 1.0)))))))
    (:`then_1`
      ;[1 1 1 1 22] Комплект нод отвечающий за подщёт врагов вокруг.
      ; Во-первых, для того, чтобы определять находиться ли актор в группе врагов.
      ; Во-вторых, в какой части группы он находиться — Group Vector
      (`KismetSystemLibrary.Delay` 0.2)
      (`|ExecutionSequence`
        (:`then_0`
          (`self.CaltulateGroup_IsInGroup&GroupVector`))
        (:`then_1`
          ;;[1 1 1] На основе GroupVector менает материал у врагов в передней части группы.
          ;; А также слегка уменьшает скорость этих авангардных врагов, для того чтобы группа меньше разбредалась.
          (if (`self.IsNowSlowed?`)
            _
            (elif (> (`KismetMathLibrary.DotProduct2D` (`self.GroupVector`) (`KismetMathLibrary.MakeVector2D` _returnvalue_x_2 _returnvalue_y_2)) -0.5)
              (set `CharacterMovementComponent.MaxWalkSpeed` 600.0 _charactermovement)
              (else
                (set `CharacterMovementComponent.MaxWalkSpeed` 500.0 _charactermovement)))))))
    (:`then_2`
      ;[1 1 1] Код, который проверяет застрял ли этот враг. Просто если не двигается.
      (`KismetSystemLibrary.Delay` 0.3)
      (`|ExecutionSequence`
        (:`then_0`
          (`KismetSystemLibrary.Delay` 0.15)
          (set `self.IsStopped` (== (stale _output_get) (`self.K2_GetActorLocation`) :`ErrorTolerance` 5.0)))
        (:`then_1`
          (bind _output_get (set `self.LocalLocation` (`self.K2_GetActorLocation`))))))
    (:`then_3`
      ;[1 1 1] Код, который пока этот враг в стане, каждыйе 0.03 секунды отталкивается от соседних врагов.
      ;
      ; Нужен для того, чтобы при толчке группы врагов в стену, они лучше распределялись в линию вдоль стены.
      (if (`self.IsInStan`)
        (`KismetSystemLibrary.Delay` 0.03)
        (`self.PushOfTheNearEnemies`)))
    (:`then_4`
      ;[1 1 1] Этот код при соприкосновении с другим врагом, телепортирует
      ; одного из них на место, пенпендикулярное второму врагу.
      ;
      ; Это создаёт структуру врагов — то, что они ходят фигурами по сеточке.
      (for _array_element (`PrimitiveComponent.GetOverlappingActors` (`self.Box`) "BP_StPanel_3_C")
        (bind _asbp_st_panel_3 (cast `/Game/Vampire-Panels/BP_StPanel_3` _array_element))
        (if (and (not (`self.IsInStan`)) (not (`self.IsStopped`)) (`self.IsActorsFrontToEachOther` _asbp_st_panel_3 self 1.2))
          (bind (_returnvalue_x_3 _returnvalue_y_3) (`KismetMathLibrary.BreakVector` (`self.K2_GetActorLocation` _asbp_st_panel_3)))
          (bind _returnvalue (- _returnvalue_y_3 _returnvalue_y))
          (bind _returnvalue_2 (- _returnvalue_x_3 _returnvalue_x))
          (`self.K2_SetActorLocation` _asbp_st_panel_3 (+ (`self.K2_GetActorLocation` _asbp_st_panel_3) (* (`KismetMathLibrary.SelectVector` (`KismetMathLibrary.MakeVector` 0.0 _returnvalue) (`KismetMathLibrary.MakeVector` _returnvalue_2) (> (`KismetMathLibrary.Sqrt` (`KismetMathLibrary.Square` _returnvalue_2)) (`KismetMathLibrary.Sqrt` (`KismetMathLibrary.Square` _returnvalue)))) -1.0)) true false))))
    (:`then_5`
      (set `self.ActualSpeed` (`KismetMathLibrary.VSize` _velocity))
      (set `self.ActualVelocity` _velocity))))

(event `self.Box.OnComponentHit`
  (params (HitComponent :type "PrimitiveComponent Object Reference") (OtherActor :type "Actor Object Reference") (OtherComp :type "PrimitiveComponent Object Reference") (NormalImpulse :type "Vector Structure") (Hit :type "HitResult Structure (by ref)"))
  ;[1 1 1] Урон по главному героою
  (bind _asbp_excavator_2 (cast `/Game/Excavator/BP_Excavator_2` OtherActor))
  (`self.PunchPlayer` _asbp_excavator_2))

(event `self.Box.OnComponentBeginOverlap`
  (params (OverlappedComponent :type "PrimitiveComponent Object Reference") (OtherActor :type "Actor Object Reference") (OtherComp :type "PrimitiveComponent Object Reference") (OtherBodyIndex :type Integer) (bFromSweep :type Boolean) (SweepResult :type "HitResult Structure (by ref)"))
  ;[1 1 1] Урон по главному героою
  (bind _asbp_excavator_2 (cast `/Game/Excavator/BP_Excavator_2` OtherActor))
  (`self.PunchPlayer` _asbp_excavator_2))

(fn `CaltulateGroup_IsInGroup&GroupVector`
  (bind _returnvalue (`self.K2_GetActorLocation`))
  (set `self.GroupVector` (0.0 0.0))
  (set `self.EnemyAround` (`|MakeArray` null :!type "/Game/Vampire-Panels/BP_StPanel_3 Object Reference"))
  (for _array_element (`PrimitiveComponent.GetOverlappingActors` (`self.GroupRadiusCollision`) "BP_StPanel_3_C")
    (bind _returnvalue_2 (`self.K2_GetActorLocation` _array_element))
    (bind (_outhit _returnvalue_3) (`KismetSystemLibrary.LineTraceSingle` :`Start` _returnvalue_2 :`End` _returnvalue :`TraceChannel` "TraceTypeQuery1" :`DrawDebugType` "ForOneFrame"))
    (if (not _returnvalue_3)
      (`KismetArrayLibrary.Array_Add` (`self.EnemyAround`) (cast `/Game/Vampire-Panels/BP_StPanel_3` _array_element :!pure true))
      (set `self.GroupVector` (+ (`KismetMathLibrary.Normal2D` (`KismetMathLibrary.MakeVector2D` (- (.x _returnvalue_2) (.x _returnvalue)) (- (.y _returnvalue_2) (.y _returnvalue)))) (`self.GroupVector`)))))
  (bind _output_get (set `self.IsInGroup` (> (`KismetArrayLibrary.Array_Length` (`self.EnemyAround`)) 9)))
  (if _output_get
    _))

(fn `PunchPlayer`
  (params (Player :type "/Game/Excavator/BP_Excavator_2 Object Reference"))
  (bind (_returnvalue_x _returnvalue_y) (`KismetMathLibrary.BreakVector` (`KismetMathLibrary.Normal` (- (`self.K2_GetActorLocation`) (`self.K2_GetActorLocation` Player)))))
  (if (`self.IsCanAttack?`)
    (`GameplayStatics.ApplyDamage` Player 1.0)
    (`/Game/Excavator/BP_Excavator_2.Pain` Player 1.0)
    (`self.LaunchCharacter` Player (* (`KismetMathLibrary.MakeVector` _returnvalue_x _returnvalue_y) -7500.0) false false)))

(fn `PushOfTheNearEnemies`
  (bind (_lastpunchvector_x _lastpunchvector_y) (`KismetMathLibrary.BreakVector` (`self.LastPunchVector`)))
  (bind _overlappingactors (`PrimitiveComponent.GetOverlappingActors` (`self.CollisionForStanHustle`) "BP_StPanel_3_C"))
  (if (> (`KismetArrayLibrary.Array_Length` _overlappingactors) 1)
    (for _array_element _overlappingactors
      (bind (_returnvalue_x _returnvalue_y) (`KismetMathLibrary.BreakVector` (* (`KismetMathLibrary.Normal` (- (`self.K2_GetActorLocation` _array_element) (`self.K2_GetActorLocation`))) -1000.0)))
      (bind _returnvalue (`KismetMathLibrary.SelectVector` (`KismetMathLibrary.MakeVector` _returnvalue_x) (`KismetMathLibrary.MakeVector` 0.0 _returnvalue_y) (< (`KismetMathLibrary.Sqrt` (`KismetMathLibrary.Square` _lastpunchvector_x)) (`KismetMathLibrary.Sqrt` (`KismetMathLibrary.Square` _lastpunchvector_y)))))
      (`self.LaunchCharacter` self _returnvalue false false)
      (`self.LaunchCharacter` (cast `/Game/Vampire-Panels/BP_StPanel_3` _array_element :!pure true) (* _returnvalue -1) false false))))

(fn `UserConstructionScript`
  (bind _constructionscript_walls (`self.ConstructionScript_Walls`))
  (`|ExecutionSequence`
    (:`then_0`
      (if (`self.ConstructionScript_IsRotated?`)
        (`SceneComponent.K2_SetRelativeRotation` (`self.HrushevkaBase`) (struct :`Yaw` 90.0) false false)))
    (:`then_1`
      (`|ExecutionSequence`
        (:`then_0`
          (`StaticMeshComponent.SetStaticMesh` (`self.Left_Wall`) (`KismetArrayLibrary.Array_Random` _constructionscript_walls) :!label _label)
          (`StaticMeshComponent.SetStaticMesh` (`self.Right_Wall`) (`KismetArrayLibrary.Array_Random` _constructionscript_walls)))
        (:`then_1`
          (if (== (`self.Right_Wall`) (`self.Left_Wall`))
            (goto _label)))))))