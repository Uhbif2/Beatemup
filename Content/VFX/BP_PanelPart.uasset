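; BP_PanelPart is a VFX actor that launches a physics-driven panel piece, apparently as flying debris.
; On BeginPlay it applies a large impulse to the PanelPart component along the actor's forward vector, with random strength and random yaw spread.
; Each Tick adds a downward impulse scaled by delta time, acting as extra gravity on the piece.
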(event `self.ReceiveBeginPlay`
  (`PrimitiveComponent.AddImpulse` (`self.Panel Part`) (`KismetMathLibrary.GreaterGreater_VectorRotator` (* (`self.GetActorForwardVector`) (`KismetMathLibrary.RandomFloatInRange` 60000.0 120000.0) 60) (`KismetMathLibrary.MakeRotator` 0.0 0.0 (`KismetMathLibrary.RandomFloatInRange` -40.0 40.0))) "None" false))

(event `self.ReceiveTick`
  (params (DeltaSeconds :type "Float (single-precision)"))
  (`PrimitiveComponent.AddImpulse` (`self.Panel Part`) (* (0.0 0.0 -300000.0) (`GameplayStatics.GetWorldDeltaSeconds`) 30.0) "None" false))

(fn `UserConstructionScript`)