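; Physics collision body for the excavator's ball that delivers hits to BP_StPanel_3 panels.
; Each tick, an impulse scaled by offset and delta time pulls component F toward the player BP_Excavator_2's CenterOfBall.
; While collision is enabled, overlapped panels receive PunchFromBall with the actor's speed and location.
; At BeginPlay, F stays physics-only for a short delay before switching to query and physics.
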(event `self.ReceiveBeginPlay`
  (`self.On\\Off Collision` false)
  (`KismetSystemLibrary.Delay` 1.0)
  (`self.On\\Off Collision` true))

(event `On\\Off Collision`
  (params (`On?` :type Boolean))
  (bind _f (`self.f`))
  (if `On?`
    (`PrimitiveComponent.SetCollisionEnabled` _f "QueryAndPhysics")
    (else
      (`PrimitiveComponent.SetCollisionEnabled` _f "PhysicsOnly"))))

(event `self.ReceiveTick`
  (params (DeltaSeconds :type "Float (single-precision)"))
  (`PrimitiveComponent.AddImpulse` (`self.f`) (* (- (`SceneComponent.K2_GetComponentLocation` (`/Game/Excavator/BP_Excavator_2.CenterOfBall` (cast `/Game/Excavator/BP_Excavator_2` (`GameplayStatics.GetPlayerCharacter` 0) :!pure true))) (`SceneComponent.K2_GetComponentLocation` (`self.f`))) (`GameplayStatics.GetWorldDeltaSeconds`) 10000000.0) "None" false)
  (if (`PrimitiveComponent.K2_IsCollisionEnabled` (`self.f`))
    (for _array_element (`PrimitiveComponent.GetOverlappingActors` (`self.f`) "/Game/Vampire-Panels/BP_StPanel_3.BP_StPanel_3_C")
      (bind _asbp_st_panel_3 (cast `/Game/Vampire-Panels/BP_StPanel_3` _array_element))
      (`/Game/Vampire-Panels/BP_StPanel_3.PunchFromBall` _asbp_st_panel_3 (`KismetMathLibrary.VSize` (`self.GetVelocity`)) (`self.K2_GetActorLocation` self)))))

(fn `UserConstructionScript`)