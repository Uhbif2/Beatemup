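; Wide kick hit-box actor that previews, then delivers an area punch to overlapping BP_StPanel_3 targets.
; Until activated, Tick keeps it ahead of the player along camera yaw, smoothly turns it by last move input and outlines targets inside.
; ActivatePunch closes that gate, freezing the box, then after a short delay tosses targets along its arrow, spawns damage decals and later destroys itself.
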(event `Activate Punch`
  (bind _returnvalue (`self.K2_GetActorRotation`))
  (bind _overlappingactors (`PrimitiveComponent.GetOverlappingActors` (`self.Box`) "/Game/Vampire-Panels/BP_StPanel_3.BP_StPanel_3_C"))
  (bind (_lastactivemovevector_x _lastactivemovevector_y) (`KismetMathLibrary.BreakVector2D` (`/Game/Excavator/BP_Excavator_2.LastActiveMoveVector` (`self.PlayerReference`))))
  (bind _returnvalue_2 (< _lastactivemovevector_y -0.2))
  (bind (_relativerotation_roll _relativerotation_pitch _relativerotation_yaw) (`KismetMathLibrary.BreakRotator` (`SceneComponent.RelativeRotation` (`/Game/Excavator/BP_Excavator_2.CameraTorsionCenter` (`self.PlayerReference`)))))
  (bind (_relativerotation_roll_2 _relativerotation_pitch_2 _relativerotation_yaw_2) (`KismetMathLibrary.BreakRotator` (`SceneComponent.RelativeRotation` (`/Game/Excavator/BP_Excavator_2.CameraTorsionCenter` (`self.PlayerReference`)))))
  (`|ExecutionSequence`
    (:`then_0`
      (`KismetSystemLibrary.Delay` 0.25)
      (`|ExecutionSequence`
        (:`then_0`
          (`KismetSystemLibrary.Delay` 1.0)
          (`self.K2_DestroyActor`))
        (:`then_1`
          (`KismetSystemLibrary.DelayUntilNextTick`)
          (set `self.Overlapping Enemys` _overlappingactors)
          (for _array_element _overlappingactors
            (bind _asbp_st_panel_3 (cast `/Game/Vampire-Panels/BP_StPanel_3` _array_element))
            (`/Game/Vampire-Panels/BP_StPanel_3.PunchWithDelay` _asbp_st_panel_3 (`KismetMathLibrary.GreaterGreater_VectorRotator` (`KismetMathLibrary.MakeVector` (* (`self.SpeedOfToss`) 5.0)) (`SceneComponent.K2_GetComponentRotation` (`self.Arrow`))) self)
            (`/Game/Vampire-Panels/BP_StPanel_3.SpawnDamageDecal` _asbp_st_panel_3 _returnvalue (+ (`KismetMathLibrary.GreaterGreater_VectorRotator` (`KismetMathLibrary.MakeVector` -220.0) _returnvalue) (`self.K2_GetActorLocation` _asbp_st_panel_3)))))))
    (:`then_1`
      (goto _label :!via `Close`))))

(event `self.ReceiveTick`
  (params (DeltaSeconds :type "Float (single-precision)"))
  (bind (_lastactivemovevector_x _lastactivemovevector_y) (`KismetMathLibrary.BreakVector2D` (`/Game/Excavator/BP_Excavator_2.LastActiveMoveVector` (`self.PlayerReference`))))
  (bind _returnvalue (< _lastactivemovevector_y -0.2))
  (bind (_relativerotation_roll _relativerotation_pitch _relativerotation_yaw) (`KismetMathLibrary.BreakRotator` (`SceneComponent.RelativeRotation` (`/Game/Excavator/BP_Excavator_2.CameraTorsionCenter` (`self.PlayerReference`)))))
  (bind (_relativerotation_roll_2 _relativerotation_pitch_2 _relativerotation_yaw_2) (`KismetMathLibrary.BreakRotator` (`SceneComponent.RelativeRotation` (`/Game/Excavator/BP_Excavator_2.CameraTorsionCenter` (`self.PlayerReference`)))))
  (`/Engine/EditorBlueprintResources/StandardMacros.Gate` false :!label _label
    (:`Exit`
      (`/Engine/EditorBlueprintResources/StandardMacros.IsValid` (`self.PlayerReference`)
        (:`Is Valid`
          (`|ExecutionSequence`
            (:`then_0`
              (if (not _returnvalue)
                (set `self.TargetRotationSwing` (`KismetMathLibrary.ComposeRotators` (`KismetMathLibrary.MakeRotator` 0.0 0.0 _relativerotation_yaw_2) (`KismetMathLibrary.SelectRotator` (struct) (`KismetMathLibrary.SelectRotator` (`KismetMathLibrary.MakeRotator` 0.0) (`KismetMathLibrary.SelectRotator` (struct :`Yaw` 90.0) (`KismetMathLibrary.SelectRotator` (struct :`Yaw` -90.0) (struct) (< _lastactivemovevector_x -0.2)) (> _lastactivemovevector_x 0.2)) _returnvalue) (> _lastactivemovevector_y 0.2))))))
            (:`then_1`
              (for _array_element (`PrimitiveComponent.GetOverlappingActors` (`self.Box`) "/Game/Vampire-Panels/BP_StPanel_3.BP_StPanel_3_C")
                (bind _asbp_st_panel_3 (cast `/Game/Vampire-Panels/BP_StPanel_3` _array_element))
                (`/Game/Vampire-Panels/BP_StPanel_3.Activate Outline` _asbp_st_panel_3 (`self.K2_GetActorRotation`))))
            (:`then_2`
              (`self.K2_SetActorRotation` (`KismetMathLibrary.RLerp` (`self.TargetRotationSwing`) (`self.K2_GetActorRotation`) 0.4 true))
              (`self.K2_SetActorLocation` (+ (`self.K2_GetActorLocation` (`self.PlayerReference`)) (* (`KismetMathLibrary.GreaterGreater_VectorRotator` (1.0 0.0 0.0) (`KismetMathLibrary.MakeRotator` 0.0 0.0 _relativerotation_yaw)) 1500.0))))))))))

(fn `UserConstructionScript`)