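; BP_LongKickBox is a temporary long-kick hit box that punches and shoves BP_StPanel_3 enemies along its arrow.
; Until ActivatePunch's delay ends, Tick box-traces from the player along camera yaw, snapping the box near the hit actor in 45-degree yaw steps.
; It then locks placement, punches overlapping enemies, and launches ungrouped ones each tick, pulling them toward the centerline to form a line.
; It destroys itself shortly afterwards.
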(event `ActivatePunch`
  (bind (_returnvalue_roll _returnvalue_pitch _returnvalue_yaw) (`KismetMathLibrary.BreakRotator` (`self.GetPuchCollisionRotation`)))
  (bind _overlappingactors (`PrimitiveComponent.GetOverlappingActors` (`self.Box`) "/Game/Vampire-Panels/BP_StPanel_3.BP_StPanel_3_C"))
  (bind (_relativelocation_x _relativelocation_y) (`KismetMathLibrary.BreakVector` (`SceneComponent.RelativeLocation` (`self.Arrow`))))
  (bind _returnvalue (`SceneComponent.K2_GetComponentLocation` (`Character.CapsuleComponent` (`self.PlayerReference`))))
  (bind (_relativerotation_roll _relativerotation_pitch _relativerotation_yaw) (`KismetMathLibrary.BreakRotator` (`SceneComponent.RelativeRotation` (`/Game/Excavator/BP_Excavator_2.CameraTorsionCenter` (`self.PlayerReference`)))))
  (bind _returnvalue_2 (`KismetMathLibrary.MakeRotator` _returnvalue_roll _returnvalue_pitch (* (`KismetMathLibrary.Round` (/ _returnvalue_yaw 45.0)) 45.0)))
  (`KismetSystemLibrary.Delay` 1.1)
  (`|ExecutionSequence`
    (:`then_0`
      (`KismetSystemLibrary.DelayUntilNextTick`)
      (set `self.Overlapping Enemys` _overlappingactors)
      (for _array_element _overlappingactors
        (bind _asbp_st_panel_3 (cast `/Game/Vampire-Panels/BP_StPanel_3` _array_element))
        (`/Game/Vampire-Panels/BP_StPanel_3.PunchWithDelay` _asbp_st_panel_3 (`KismetMathLibrary.GreaterGreater_VectorRotator` (`KismetMathLibrary.MakeVector` 1.0) (`SceneComponent.K2_GetComponentRotation` (`self.Arrow`))) null)))
    (:`then_1`
      (`KismetSystemLibrary.Delay` 1.4)
      (`self.K2_DestroyActor`))
    (:`then_2`
      (goto _label :!via `Open`))
    (:`then_3`
      (goto _label_2 :!via `Close`))))

(event `self.ReceiveTick`
  (params (DeltaSeconds :type "Float (single-precision)"))
  (bind (_returnvalue_roll _returnvalue_pitch _returnvalue_yaw) (`KismetMathLibrary.BreakRotator` (`self.GetPuchCollisionRotation`)))
  (bind (_relativelocation_x _relativelocation_y) (`KismetMathLibrary.BreakVector` (`SceneComponent.RelativeLocation` (`self.Arrow`))))
  (bind _returnvalue (`SceneComponent.K2_GetComponentLocation` (`Character.CapsuleComponent` (`self.PlayerReference`))))
  (bind (_relativerotation_roll _relativerotation_pitch _relativerotation_yaw) (`KismetMathLibrary.BreakRotator` (`SceneComponent.RelativeRotation` (`/Game/Excavator/BP_Excavator_2.CameraTorsionCenter` (`self.PlayerReference`)))))
  (bind _returnvalue_2 (`KismetMathLibrary.MakeRotator` _returnvalue_roll _returnvalue_pitch (* (`KismetMathLibrary.Round` (/ _returnvalue_yaw 45.0)) 45.0)))
  (`|ExecutionSequence`
    (:`then_0`
      ;[1 1 1] Код отвечающий за толкание в определённом направлении.
      ;
      ; А также если толкаемы враг не на оси этого актора — то этот код толкает врага к центру. То есть стаблизирует линию врагов в линию.
      (`/Engine/EditorBlueprintResources/StandardMacros.Gate` true :!label _label
        (:`Exit`
          (if (not (`KismetArrayLibrary.Array_IsEmpty` (`self.Overlapping Enemys`)))
            (for _array_element (`self.Overlapping Enemys`)
              (if (`PrimitiveComponent.IsOverlappingActor` (`self.Box`) _array_element)
                (bind _asbp_st_panel_3 (cast `/Game/Vampire-Panels/BP_StPanel_3` _array_element :!pure true))
                (if (not (`/Game/Vampire-Panels/BP_StPanel_3.IsInGroup` _asbp_st_panel_3))
                  (bind (_returnvalue_x _returnvalue_y) (`KismetMathLibrary.BreakVector` (`KismetMathLibrary.InverseTransformLocation` (`self.GetTransform`) (`self.K2_GetActorLocation` _array_element))))
                  (bind _returnvalue_3 (- _returnvalue_y _relativelocation_y))
                  (`Character.LaunchCharacter` _asbp_st_panel_3 (* (`KismetMathLibrary.GreaterGreater_VectorRotator` (`KismetMathLibrary.MakeVector` (`self.SpeedOfToss`) (`KismetMathLibrary.SelectFloat` 0.0 (* _returnvalue_3 -1.0 10.0) (== _returnvalue_3 0.0))) (`SceneComponent.K2_GetComponentRotation` (`self.Arrow`))) (`GameplayStatics.GetWorldDeltaSeconds`) 100.0) false false))
                (else
                  (`KismetArrayLibrary.Array_RemoveItem` (`self.Overlapping Enemys`) _array_element))))))))
    (:`then_1`
      (`/Engine/EditorBlueprintResources/StandardMacros.Gate` false :!label _label_2
        (:`Exit`
          (`/Engine/EditorBlueprintResources/StandardMacros.IsValid` (`self.PlayerReference`)
            (:`Is Valid`
              (bind (_outhit _returnvalue_4) (`KismetSystemLibrary.BoxTraceSingle` _returnvalue (+ _returnvalue (`KismetMathLibrary.GreaterGreater_VectorRotator` (`KismetMathLibrary.MakeVector` 5000.0) (`KismetMathLibrary.MakeRotator` 0.0 0.0 _relativerotation_yaw))) (30.0 1500.0 1000.0) (`KismetMathLibrary.MakeRotator` 0.0 0.0 _relativerotation_yaw) "TraceTypeQuery3"))
              (`|ExecutionSequence`
                (:`then_2`
                  (if _returnvalue_4
                    (`self.K2_SetActorLocationAndRotation` (+ (* (`KismetMathLibrary.GreaterGreater_VectorRotator` (1.0 0.0 0.0) _returnvalue_2) 2500.0) (`self.K2_GetActorLocation` (`.HitActor` (`GameplayStatics.BreakHitResult` _outhit)))) _returnvalue_2)))))))))))

(fn `UserConstructionScript`)