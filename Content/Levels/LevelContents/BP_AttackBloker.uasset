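; BP_AttackBloker is a level-placed box volume that blocks selected attacks of a BP_Excavator_2.
; Shortly after BeginPlay it takes the first overlapping excavator and sets its blocked flags for long attack, wide attack and ball put-down, as enabled by the volume's booleans.
; End overlap clears those flags, while begin overlap only casts, so later entry sets nothing.
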(event `self.ReceiveBeginPlay`
  (`KismetSystemLibrary.Delay` 0.2)
  (bind _asbp_excavator_2 (cast `/Game/Excavator/BP_Excavator_2` (`|GetArrayItem` (`PrimitiveComponent.GetOverlappingActors` (`self.Box`) "/Game/Excavator/BP_Excavator_2.BP_Excavator_2_C"))))
  (`|ExecutionSequence`
    (:`then_0`
      (if (`self.IsBlockLongAttack`)
        (set `/Game/Excavator/BP_Excavator_2.IsBlockedLongAttack` true _asbp_excavator_2)))
    (:`then_1`
      (if (`self.IsBlockPuttingDownBall`)
        (set `/Game/Excavator/BP_Excavator_2.IsBlockedBallPutDown?` true _asbp_excavator_2)))
    (:`then_2`
      (if (`self.IsBlockWideAttack`)
        (set `/Game/Excavator/BP_Excavator_2.IsBlockedWideAttack` true _asbp_excavator_2)))))

(event `self.Box.OnComponentBeginOverlap`
  (params (OverlappedComponent :type "PrimitiveComponent Object Reference") (OtherActor :type "Actor Object Reference") (OtherComp :type "PrimitiveComponent Object Reference") (OtherBodyIndex :type Integer) (bFromSweep :type Boolean) (SweepResult :type "HitResult Structure (by ref)"))
  (bind _asbp_excavator_2 (cast `/Game/Excavator/BP_Excavator_2` OtherActor)))

(event `self.Box.OnComponentEndOverlap`
  (params (OverlappedComponent :type "PrimitiveComponent Object Reference") (OtherActor :type "Actor Object Reference") (OtherComp :type "PrimitiveComponent Object Reference") (OtherBodyIndex :type Integer))
  (bind _asbp_excavator_2 (cast `/Game/Excavator/BP_Excavator_2` OtherActor))
  (`|ExecutionSequence`
    (:`then_0`
      (if (`self.IsBlockLongAttack`)
        (set `/Game/Excavator/BP_Excavator_2.IsBlockedLongAttack` false _asbp_excavator_2)))
    (:`then_1`
      (if (`self.IsBlockPuttingDownBall`)
        (set `/Game/Excavator/BP_Excavator_2.IsBlockedBallPutDown?` false _asbp_excavator_2)))
    (:`then_2`
      (if (`self.IsBlockWideAttack`)
        (set `/Game/Excavator/BP_Excavator_2.IsBlockedWideAttack` false _asbp_excavator_2)))))

(fn `UserConstructionScript`)