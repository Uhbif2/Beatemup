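; BP_OpenTutorialText is a level trigger that shows a tutorial text widget with configurable text and time.
; A BP_Excavator_2 entering the Box creates the WB_TutorialText widget and adds it to the viewport.
; If the excavator is already inside shortly after BeginPlay, it is given a StartGameAfterStory callback that shows the same widget.
; A DoOnce shared by both paths limits the tutorial to one display.
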(event `self.ReceiveBeginPlay`
  (bind _overlappingactors (`PrimitiveComponent.GetOverlappingActors` (`self.Box`) "/Game/Excavator/BP_Excavator_2.BP_Excavator_2_C"))
  (`KismetSystemLibrary.Delay` 0.1)
  (if (not (`KismetArrayLibrary.Array_IsEmpty` _overlappingactors))
    (bind _asbp_excavator_2 (cast `/Game/Excavator/BP_Excavator_2` (`|GetArrayItem` _overlappingactors)))
    (add `/Game/Excavator/BP_Excavator_2.StartGameAfterStory` _asbp_excavator_2 (delegate `StartGameAfterStory_Event`))))

(event `StartGameAfterStory_Event`
  (`/Engine/EditorBlueprintResources/StandardMacros.DoOnce` false :!label _label
    (:`Completed`
      (bind _returnvalue (`|CreateWidget` "/Game/Interface/WB_TutorialText.WB_TutorialText_C" null (`self.Text`) (`self.Time`)))
      (`UserWidget.AddToViewport` _returnvalue 0))))

(event `self.Box.OnComponentBeginOverlap`
  (params (OverlappedComponent :type "PrimitiveComponent Object Reference") (OtherActor :type "Actor Object Reference") (OtherComp :type "PrimitiveComponent Object Reference") (OtherBodyIndex :type Integer) (bFromSweep :type Boolean) (SweepResult :type "HitResult Structure (by ref)"))
  (cast `/Game/Excavator/BP_Excavator_2` OtherActor)
  (goto _label))

(fn `UserConstructionScript`)