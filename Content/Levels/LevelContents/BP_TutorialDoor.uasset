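; Tutorial door that falls open once its target enemies are gone and enough have been fed to a fire stove.
; BeginPlay saves enemy start locations and binds the check to the stoves' fired-enemy events.
; A met quota, or disabled respawn, triggers a one-time timeline fall with collision removal, sound and camera shake.
; Otherwise, it respawns BP_DeadPanel enemies at saved locations behind a screen fade and shows tutorial text.
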(event `RespawnTargetEnemies`
  (for (_ _array_index) (`self.TargetDepthActors`)
    (bind _returnvalue (`|SpawnActorFromClass` "/Game/Vampire-Panels/BP_DeadPanel.BP_DeadPanel_C" (`KismetMathLibrary.MakeTransform` (`|GetArrayItem` (`self.EnemiesStartLocations`) _array_index)) "Undefined" "MultiplyWithRoot" null true null))
    (`KismetArrayLibrary.Array_Set` (`self.TargetDepthActors`) _array_index _returnvalue))
  (bind _returnvalue_2 (`|CreateWidget` "/Game/Interface/WB_FadeOut.WB_FadeOut_C"))
  (`UserWidget.AddToViewport` _returnvalue_2 0))

(event `self.ReceiveBeginPlay`
  (bind _targetfirestove_1 (`self.TargetFireStove_1`))
  (`|ExecutionSequence`
    (:`then_0`
      (for (_array_element _array_index) (`self.TargetDepthActors`)
        (`/Engine/EditorBlueprintResources/StandardMacros.IsValid` _array_element
          (:`Is Valid`
            (`KismetArrayLibrary.Array_Set` (`self.EnemiesStartLocations`) _array_index (`self.K2_GetActorLocation` _array_element))))))
    (:`then_1`
      (for _array_element_2 (`self.TargetFireStove_2(If Not Respawn)`)
        (`/Engine/EditorBlueprintResources/StandardMacros.IsValid` _array_element_2
          (:`Is Valid`
            (add `/Game/Oven/BP_Oven.FiredEnemies` _array_element_2 (delegate `CheckIsTargetEnemiesFired`))))))
    (:`then_2`
      (`/Engine/EditorBlueprintResources/StandardMacros.IsValid` _targetfirestove_1
        (:`Is Valid`
          (add `/Game/Oven/BP_Oven.FiredEnemies` _targetfirestove_1 (delegate `CheckIsTargetEnemiesFired`)))))))

(event `CheckIsTargetEnemiesFired`
  (set `self.LocalCounter` false)
  (for _array_element (`self.TargetDepthActors`)
    (set `self.LocalCounter` (or (`self.LocalCounter`) (`KismetSystemLibrary.IsValid` _array_element))))
  (if (`self.LocalCounter`)
    _
    (elif (>= (`/Game/Oven/BP_Oven.HowMuchEnemy` (`self.TargetFireStove_1`)) (`self.CountEnemyTargetToNOTRespawn`))
      (`/Engine/EditorBlueprintResources/StandardMacros.DoOnce` false :!label _label
        (:`Completed`
          (bind (_direction _newtrack_0) (`Timeline|Timeline` :!via `PlayFromStart`)
            (:`Update`
              (`SceneComponent.K2_SetRelativeRotation` (`self.Cube`) (`KismetMathLibrary.RLerp` (struct) (`KismetMathLibrary.SelectRotator` (struct :`Roll` -90.0) (struct :`Roll` 90.0) (`self.AnoutherSideFall`)) _newtrack_0 true) false false))
            (:`Finished`
              (`PrimitiveComponent.SetCollisionEnabled` (`self.Cube`) "NoCollision")
              (`GameplayStatics.PlaySound2D` "/Game/Sounds/AttackWithBreak.AttackWithBreak" 1.0 1.0 0.0 null null)
              (`GameplayStatics.PlayWorldCameraShake` "/Game/Excavator/CmSh_Damage.CmSh_Damage_C" (`SceneComponent.K2_GetComponentLocation` (`/Game/Excavator/BP_Excavator_2.FollowCamera` (cast `/Game/Excavator/BP_Excavator_2` (`GameplayStatics.GetPlayerCharacter` 0) :!pure true))) 500.0 500.0)))))
      (elif (not (`self.IsWithRespawn?`))
        (goto _label)
        (else
          (bind _returnvalue (`|CreateWidget` "/Game/Interface/WB_FadeIn.WB_FadeIn_C"))
          (`UserWidget.AddToViewport` _returnvalue 0)
          (`KismetSystemLibrary.Delay` 0.2)
          (`self.RespawnTargetEnemies`)
          (bind _returnvalue_2 (`|CreateWidget` "/Game/Interface/WB_TutorialText.WB_TutorialText_C" null "08" 12.0))
          (`UserWidget.AddToViewport` _returnvalue_2 0))))))

(fn `UserConstructionScript`)